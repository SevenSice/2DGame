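; BP_UnityChan is a 2D side-scrolling player character that moves along X, jumps and plays Paper2D flipbook animations.
; Tick maps the State enum to a sprite flipbook and yaws the controller to face horizontal velocity, or the last input direction when stationary.
; Jump input sets an air state from vertical velocity; landing shows a brief landing state, then picks Running or Idle.
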(event Custom|UpdateAnimation
  (Sprite|SetFlipbook (Variables|Default|GetSprite) (Utilities|Select :Index (Variables|Default|GetState) :NewEnumerator0 "/Game/MyFile/Sprites/unityChan/Normal/Unitychan_Idle.Unitychan_Idle" :NewEnumerator1 "/Game/MyFile/Sprites/unityChan/Normal/Unitychan_Walk.Unitychan_Walk" :NewEnumerator2 "/Game/MyFile/Sprites/unityChan/Battle/Unitychan_Run.Unitychan_Run" :NewEnumerator3 "/Game/MyFile/Sprites/unityChan/Normal/Unitychan_Jump_Up.Unitychan_Jump_Up" :NewEnumerator4 "/Game/MyFile/Sprites/unityChan/Normal/Unitychan_Jump_MidAir.Unitychan_Jump_MidAir" :NewEnumerator5 "/Game/MyFile/Sprites/unityChan/Normal/Unitychan_Jump_Fall.Unitychan_Jump_Fall" :NewEnumerator6 "/Game/MyFile/Sprites/unityChan/Normal/Unitychan_Jump_Landing_Flipbook.Unitychan_Jump_Landing_Flipbook" :NewEnumerator7 0)))

(event Custom|ForwardDirection
  ;[1 1 1] Forward Direction
)

(event EventBeginPlay
  (Class|ActorComponent|SetIsReplicated (Variables|Default|GetSprite) true))

(event Collision|EventActorBeginOverlap
  (params (OtherActor :type Actor%20Object%20Reference)))

(event EventTick
  (params (DeltaSeconds :type Float%20%28single-precision%29))
  ;[1 1 1] Forward Direction
  (Utilities|FlowControl|Sequence
    (:then_0
      (CallFunction|UpdateAnimation)
      (Math|Float|CompareFloat (.X (Math|Vector|BreakVector (Variables|/Script/Engine.MovementComponent|GetVelocity (Pawn|GetMovementComponent)))) 0.0
        (:>
          (Pawn|SetControlRotation (Pawn|GetController) (Math|Rotator|MakeRotator 0.0 0.0 0.0) :!label _label))
        (:==
          (if (Variables|Default|GetBisMoveingRight)
            (goto _label)
            (else
              (Pawn|SetControlRotation (Pawn|GetController) (Math|Rotator|MakeRotator 0.0 0.0 1.8e+02) :!label _label_2))))
        (:<
          (goto _label_2))))))

(event EventOnLanded
  (params (Hit :type Hit%20Result%20Structure%20%28by%20ref%29))
  (Variables|Default|SetState "NewEnumerator6")
  (Utilities|FlowControl|Delay 0.1)
  (if (not (Variables|Default|GetIsHit?))
    (if (> (.z (Transformation|GetVelocity)) 0.0)
      (Variables|Default|SetState "NewEnumerator2")
      (else
        (Variables|Default|SetState "NewEnumerator0")))))

(event Input|ActionEvents|InputActionJump
  (params (Key :type Key%20Structure))
  (:Pressed
    (Character|Jump)
    (Math|Float|CompareFloat (.Z (Math|Vector|BreakVector (Variables|/Script/Engine.MovementComponent|GetVelocity (Variables|Character|GetCharacterMovement)))) 0.0
      (:>
        (Variables|Default|SetState "NewEnumerator3"))
      (:==
        (Variables|Default|SetState "NewEnumerator4"))
      (:<
        (Variables|Default|SetState "NewEnumerator5"))))
  (:Released
    (Character|StopJumping)))

(event Input|AxisEvents|InputAxisMoveRight
  (params (AxisValue :type Float%20%28single-precision%29))
  ;[1 1 1] MoveRight
  (if (not (Variables|Default|GetCanMove?))
    (if (> AxisValue 0.0)
      (Variables|Default|SetBisMoveingRight true)
      (elif (< AxisValue 0.0)
        (Variables|Default|SetBisMoveingRight false)))
    (Pawn|Input|AddMovementInput "1.000000, 0, 0" AxisValue false)))

(fn ConstructionScript)