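; Map pawn that acts as a level-select camera, moving between points of interest (POIs) in the world.
; It starts at the first POI, and cycle inputs step CurrentPOI forward or back with wraparound, teleporting the pawn to that POI.
; The Shoot input opens the level named on the current POI.
; A debug-style 1 key toggles the camera between perspective and orthographic projection.
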(event EventBeginPlay
  (Transformation|SetActorLocation (Transformation|GetActorLocation (Utilities|Array|Get(acopy) (Variables|Default|GetPOIs))) false false))

(event Collision|EventActorBeginOverlap
  (params (OtherActor :type Actor%20Object%20Reference)))

(event EventTick
  (params (DeltaSeconds :type Float%20%28single-precision%29)))

(event Input|ActionEvents|InputActionCycleForward
  (params (Key :type Key%20Structure))
  (:Pressed
    (bind _output_get (Variables|Default|SetCurrentPOI (Math|Integer|%(Integer) (+ (Variables|Default|GetCurrentPOI) 1) (Utilities|Array|Length (Variables|Default|GetPOIs)))))
    (CallFunction|SetCameraPawnLocation _output_get)))

(event Input|ActionEvents|InputActionCycleBack
  (params (Key :type Key%20Structure))
  (:Pressed
    (if (< (- (Variables|Default|GetCurrentPOI) 1) 0)
      (bind _output_get (Variables|Default|SetCurrentPOI (- (Utilities|Array|Length (Variables|Default|GetPOIs)) 1)))
      (CallFunction|SetCameraPawnLocation _output_get)
      (else
        (bind _output_get_2 (Variables|Default|SetCurrentPOI (- (Variables|Default|GetCurrentPOI) 1)))
        (CallFunction|SetCameraPawnLocation _output_get_2)))))

(event Input|ActionEvents|InputActionShoot
  (params (Key :type Key%20Structure))
  (:Pressed
    (Game|OpenLevel(byName) (Variables|/Game/MyFile/BP/POI.POI_C|GetLevelToOpen (Utilities|Array|Get(acopy) (Variables|Default|GetPOIs) (Variables|Default|GetCurrentPOI))))))

(event Input|KeyboardEvents|1
  (params (Key :type Key%20Structure))
  (bind _camera (Variables|Default|GetCamera))
  (:Pressed
    (Utilities|FlowControl|FlipFlop
      (:A
        (Class|CameraComponent|SetProjectionMode _camera "Perspective"))
      (:B
        (Class|CameraComponent|SetProjectionMode _camera "Orthographic")
        (Development|PrintString "Hello")))))

(fn ConstructionScript)

(fn SetCameraPawnLocation
  (params (Dimension%201 :type Integer))
  (Transformation|SetActorLocation (Transformation|GetActorLocation (Utilities|Array|Get(acopy) (Variables|Default|GetPOIs) Dimension%201)) false false))